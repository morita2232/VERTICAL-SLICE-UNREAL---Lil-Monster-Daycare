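; Level 1 shift clock and end-of-level scorer that shows timer and final-score widgets.
; A looping one-minute timer advances the displayed clock an hour from an 8 A.M. base, showing noon as 0:00 P.M.
; At TotalMinutes it stops and totals Boredom, Anger and Hunger across five baby monster and human classes.
; The per-baby average is printed, then the hidden score widget's ShowScores is called.
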(event Custom|AdvanceTime
  (bind _timerlevel1 (Variables|Default|GetTimerLevel1))
  (bind _output_get (Variables|Default|SetelapsedMinutes (+ (Variables|Default|GetelapsedMinutes) 1)))
  (if (>= (+ _output_get 8) 12)
    (Rendering|Components|TextRender|SetText (Variables|/Game/VERTICAL_SLICE/BLUEPRINTS/HUDS/WBP_TimeLevel1.WBP_TimeLevel1_C|GetRichTextBlock_53 _timerlevel1) (Utilities|Text|ToText(String) (Utilities|String|Append (Utilities|String|ToString(Integer) (- (+ (Variables|Default|GetelapsedMinutes) 8) 12)) ":00 P.M")))
    (else
      (Rendering|Components|TextRender|SetText (Variables|/Game/VERTICAL_SLICE/BLUEPRINTS/HUDS/WBP_TimeLevel1.WBP_TimeLevel1_C|GetRichTextBlock_53 _timerlevel1) (Utilities|Text|ToText(String) (Utilities|String|Append (Utilities|String|ToString(Integer) (+ _output_get 8)) ":00 A.M")))))
  (if (>= _output_get (Variables|Default|GetTotalMinutes))
    (CallFunction|CalculateScore)
    (Utilities|Time|ClearandInvalidateTimerbyHandle (stale EventBeginPlay _returnvalue_3))))

(event Custom|CalculateScore
  (Variables|Default|SetTotalHumans 0)
  (Variables|Default|SetHumanScore 0.0)
  (Variables|Default|SetTotalSlimes 0)
  (Variables|Default|SetSlimeScore 0.0)
  (Variables|Default|SetTotalVampires 0)
  (Variables|Default|SetVampireScore 0.0)
  (Variables|Default|SetTotalWereWolves 0)
  (Variables|Default|SetWereWolfScore 0.0)
  (Variables|Default|SetTotalZombies 0)
  (Variables|Default|SetZombieScore 0.0)
  (bind _outactors (Actor|GetAllActorsOfClass "/Game/VERTICAL_SLICE/BLUEPRINTS/BABIES/BP_BabyHuman.BP_BabyHuman_C"))
  (for _array_element _outactors
    (Variables|Default|SetTotalHumans (+ (Variables|Default|GetTotalHumans) 1))
    (Variables|Default|SetHumanScore (+ (+ (Variables|/Game/VERTICAL_SLICE/BLUEPRINTS/BABIES/BP_Baby.BP_Baby_C|GetBoredom _array_element) (Variables|/Game/VERTICAL_SLICE/BLUEPRINTS/BABIES/BP_Baby.BP_Baby_C|GetAnger _array_element) (Variables|/Game/VERTICAL_SLICE/BLUEPRINTS/BABIES/BP_Baby.BP_Baby_C|GetHunger _array_element)) (Variables|Default|GetHumanScore))))
  (bind _outactors_2 (Actor|GetAllActorsOfClass "/Game/VERTICAL_SLICE/BLUEPRINTS/BABIES/BP_BabySlime.BP_BabySlime_C"))
  (for _array_element_2 _outactors_2
    (Variables|Default|SetTotalSlimes (+ (Variables|Default|GetTotalSlimes) 1))
    (Variables|Default|SetSlimeScore (+ (+ (Variables|/Game/VERTICAL_SLICE/BLUEPRINTS/BABIES/BP_Baby.BP_Baby_C|GetBoredom _array_element_2) (Variables|/Game/VERTICAL_SLICE/BLUEPRINTS/BABIES/BP_Baby.BP_Baby_C|GetAnger _array_element_2) (Variables|/Game/VERTICAL_SLICE/BLUEPRINTS/BABIES/BP_Baby.BP_Baby_C|GetHunger _array_element_2)) (Variables|Default|GetSlimeScore))))
  (bind _outactors_3 (Actor|GetAllActorsOfClass "/Game/VERTICAL_SLICE/BLUEPRINTS/BABIES/BP_BabyVampire.BP_BabyVampire_C"))
  (for _array_element_3 _outactors_3
    (Variables|Default|SetTotalVampires (+ (Variables|Default|GetTotalVampires) 1))
    (Variables|Default|SetVampireScore (+ (+ (Variables|/Game/VERTICAL_SLICE/BLUEPRINTS/BABIES/BP_Baby.BP_Baby_C|GetBoredom _array_element_3) (Variables|/Game/VERTICAL_SLICE/BLUEPRINTS/BABIES/BP_Baby.BP_Baby_C|GetAnger _array_element_3) (Variables|/Game/VERTICAL_SLICE/BLUEPRINTS/BABIES/BP_Baby.BP_Baby_C|GetHunger _array_element_3)) (Variables|Default|GetVampireScore))))
  (bind _outactors_4 (Actor|GetAllActorsOfClass "/Game/VERTICAL_SLICE/BLUEPRINTS/BABIES/BP_BabyWereWolf.BP_BabyWereWolf_C"))
  (for _array_element_4 _outactors_4
    (Variables|Default|SetTotalWereWolves (+ (Variables|Default|GetTotalWereWolves) 1))
    (Variables|Default|SetWereWolfScore (+ (+ (Variables|/Game/VERTICAL_SLICE/BLUEPRINTS/BABIES/BP_Baby.BP_Baby_C|GetBoredom _array_element_4) (Variables|/Game/VERTICAL_SLICE/BLUEPRINTS/BABIES/BP_Baby.BP_Baby_C|GetAnger _array_element_4) (Variables|/Game/VERTICAL_SLICE/BLUEPRINTS/BABIES/BP_Baby.BP_Baby_C|GetHunger _array_element_4)) (Variables|Default|GetWereWolfScore))))
  (bind _outactors_5 (Actor|GetAllActorsOfClass "/Game/VERTICAL_SLICE/BLUEPRINTS/BABIES/BP_BabyZombie.BP_BabyZombie_C"))
  (for _array_element_5 _outactors_5
    (Variables|Default|SetTotalZombies (+ (Variables|Default|GetTotalZombies) 1))
    (Variables|Default|SetZombieScore (+ (+ (Variables|/Game/VERTICAL_SLICE/BLUEPRINTS/BABIES/BP_Baby.BP_Baby_C|GetBoredom _array_element_5) (Variables|/Game/VERTICAL_SLICE/BLUEPRINTS/BABIES/BP_Baby.BP_Baby_C|GetAnger _array_element_5) (Variables|/Game/VERTICAL_SLICE/BLUEPRINTS/BABIES/BP_Baby.BP_Baby_C|GetHunger _array_element_5)) (Variables|Default|GetZombieScore))))
  (Variables|Default|SetFinalScore (+ (Variables|Default|GetHumanScore) (Variables|Default|GetSlimeScore) (Variables|Default|GetVampireScore) (Variables|Default|GetWereWolfScore) (Variables|Default|GetZombieScore)))
  (Variables|Default|SetTotalBabies (Math|Conversions|ToFloat(Integer) (+ (Variables|Default|GetTotalHumans) (Variables|Default|GetTotalSlimes) (Variables|Default|GetTotalVampires) (Variables|Default|GetTotalWereWolves) (Variables|Default|GetTotalZombies))))
  (bind _output_get (Variables|Default|SetActualScore (/ (Variables|Default|GetFinalScore) (Variables|Default|GetTotalBabies))))
  (Development|PrintString (Utilities|String|Append "Score: " (Utilities|String|ToString(Float) _output_get)) true true "(R=0.268052,G=0.000000,B=1.000000,A=1.000000)" 5e+01)
  (Default|ShowScores (Variables|Default|GetScoreShowcaseLevel1)))

(event EventBeginPlay
  (bind _returnvalue (UserInterface|CreateWidget "/Game/VERTICAL_SLICE/BLUEPRINTS/HUDS/WBP_FinalScoreLevel1.WBP_FinalScoreLevel1_C"))
  (Variables|Default|SetScoreShowcaseLevel1 _returnvalue)
  (UserInterface|Viewport|AddtoViewport _returnvalue 0)
  (Widget|SetVisibility (Variables|Default|GetScoreShowcaseLevel1) "Hidden")
  (bind _returnvalue_2 (UserInterface|CreateWidget "/Game/VERTICAL_SLICE/BLUEPRINTS/HUDS/WBP_TimeLevel1.WBP_TimeLevel1_C"))
  (Variables|Default|SetTimerLevel1 _returnvalue_2)
  (UserInterface|Viewport|AddtoViewport _returnvalue_2 0)
  (Widget|SetVisibility (Variables|Default|GetTimerLevel1) "Visible")
  (bind _returnvalue_3 (Utilities|Time|SetTimerbyEvent (delegate Custom|AdvanceTime) 6e+01 true))
  (Utilities|FlowControl|Delay 5.0)
  (Widget|SetVisibility (Variables|/Game/VERTICAL_SLICE/BLUEPRINTS/HUDS/WBP_TimeLevel1.WBP_TimeLevel1_C|GetStartText (Variables|Default|GetTimerLevel1)) "Hidden"))

(fn ConstructionScript)