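; Level 1 baby spawn zone that populates the level with BP_BabyHuman actors up to a MaxBabies cap.
; From BeginPlay, SpawnBaby loops through random delays, spawning each baby at a randomly selected SpawnLocations entry and incrementing CurrentBabies.
; The random index never reaches the fifth wired location, and the cached mesh location SpawnLoc goes unused.
; At the cap, it prints a message to keep the babies alive.
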(event Custom|SpawnBaby
  (if (< (Variables|Default|GetCurrentBabies) (Variables|Default|GetMaxBabies)) :!label _label
    (Utilities|FlowControl|Delay (Math|Random|RandomFloatinRange 1.0 1e+01))
    (Game|SpawnActorfromClass "/Game/VERTICAL_SLICE/BLUEPRINTS/BABIES/BP_BabyHuman.BP_BabyHuman_C" (Math|Transform|MakeTransform (Utilities|Select :Index (Math|Random|RandomInteger 4) :Option%200 (Utilities|Array|Get(acopy) (Variables|Default|GetSpawnLocations)) :Option%201 (Utilities|Array|Get(acopy) (Variables|Default|GetSpawnLocations) 1) :Option%202 (Utilities|Array|Get(acopy) (Variables|Default|GetSpawnLocations) 2) :Option%203 (Utilities|Array|Get(acopy) (Variables|Default|GetSpawnLocations) 3) :Option%204 (Utilities|Array|Get(acopy) (Variables|Default|GetSpawnLocations) 4)) "0, 0, 0" "1.000000,1.000000,1.000000") "Undefined" "MultiplyWithRoot" 0 0)
    (Variables|Default|SetCurrentBabies (+ (Variables|Default|GetCurrentBabies) 1))
    (goto _label)
    (else
      (Development|PrintString "All babies are here! KEEP THEM ALIVE"))))

(event EventBeginPlay
  (Variables|Default|SetSpawnLoc (Transformation|GetWorldLocation (Variables|Default|GetStaticMesh)))
  (CallFunction|SpawnBaby))

(fn ConstructionScript)