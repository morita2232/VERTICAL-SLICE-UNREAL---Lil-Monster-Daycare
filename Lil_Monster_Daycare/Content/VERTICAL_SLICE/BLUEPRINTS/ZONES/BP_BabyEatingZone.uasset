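; BP_BabyEatingZone is a box trigger zone that feeds a BP_Baby that overlaps it, raising its Hunger value.
; Begin and end overlap set Inside and call FillingUp, which flags the baby as eating and adds FillRate on a delayed loop until MaxHunger.
; Reaching the cap sets Full, which is never reset here.
; The loop does not recheck Inside, and leaving does not clear IsEating.
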(event OnComponentBeginOverlap(Box)
  (params (OverlappedComponent :type Primitive%20Component%20Object%20Reference) (OtherActor :type Actor%20Object%20Reference) (OtherComp :type Primitive%20Component%20Object%20Reference) (OtherBodyIndex :type Integer) (bFromSweep :type Boolean) (SweepResult :type Hit%20Result%20Structure%20%28by%20ref%29))
  (if (Utilities|ClassIsChildOf (Utilities|GetClass OtherActor) "/Game/VERTICAL_SLICE/BLUEPRINTS/BABIES/BP_Baby.BP_Baby_C")
    (Variables|Default|SetBaby OtherActor)
    (Variables|Default|SetbInside true)
    (CallFunction|FillingUp)))

(event OnComponentEndOverlap(Box)
  (params (OverlappedComponent :type Primitive%20Component%20Object%20Reference) (OtherActor :type Actor%20Object%20Reference) (OtherComp :type Primitive%20Component%20Object%20Reference) (OtherBodyIndex :type Integer))
  (if (Utilities|ClassIsChildOf (Utilities|GetClass OtherActor) "/Game/VERTICAL_SLICE/BLUEPRINTS/BABIES/BP_Baby.BP_Baby_C")
    (Variables|Default|SetbInside false)
    (CallFunction|FillingUp)))

(event Custom|Filling%20Up
  (if (Variables|Default|GetbInside) :!label _label
    (if (Variables|Default|GetbFull)
      (bind _asbp_baby (Utilities|Casting|CastToBP_Baby (Variables|Default|GetBaby)))
      (Variables|/Game/VERTICAL_SLICE/BLUEPRINTS/BABIES/BP_Baby.BP_Baby_C|SetbIsEating _asbp_baby false)
      (Development|PrintString "Baby is full!")
      (else
        (bind _asbp_baby_2 (Utilities|Casting|CastToBP_Baby (Variables|Default|GetBaby) :!label _label_2))
        (Variables|/Game/VERTICAL_SLICE/BLUEPRINTS/BABIES/BP_Baby.BP_Baby_C|SetbIsEating _asbp_baby_2 true)
        (bind _output_get (Variables|/Game/VERTICAL_SLICE/BLUEPRINTS/BABIES/BP_Baby.BP_Baby_C|SetHunger _asbp_baby_2 (+ (Variables|/Game/VERTICAL_SLICE/BLUEPRINTS/BABIES/BP_Baby.BP_Baby_C|GetHunger _asbp_baby_2) (Variables|Default|GetfillRate))))
        (Utilities|FlowControl|Delay 15.0)
        (if (< _output_get (Variables|Default|GetmaxHunger))
          (Development|PrintString "Baby eating....")
          (goto _label_2)
          (else
            (Variables|Default|SetbFull true)
            (goto _label)))))
    (else
      (Development|PrintString "Baby left eating zone"))))

(fn ConstructionScript)