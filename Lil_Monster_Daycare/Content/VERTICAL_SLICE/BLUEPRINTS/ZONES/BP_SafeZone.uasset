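; BP_SafeZone is a trigger zone that relocates baby actors when they enter it.
; On box overlap it checks whether the other actor's class derives from BP_Baby, then teleports it without sweep to the SafeZone location.
; Yellow on-screen debug prints report the actor name, its class and the result of the check.
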(event OnComponentBeginOverlap(Box)
  (params (OverlappedComponent :type Primitive%20Component%20Object%20Reference) (OtherActor :type Actor%20Object%20Reference) (OtherComp :type Primitive%20Component%20Object%20Reference) (OtherBodyIndex :type Integer) (bFromSweep :type Boolean) (SweepResult :type Hit%20Result%20Structure%20%28by%20ref%29))
  (bind _returnvalue (Utilities|GetClass OtherActor))
  (Development|PrintString (Utilities|GetDisplayName OtherActor) true true "(R=1.000000,G=0.993354,B=0.000000,A=1.000000)" 2e+01)
  (Development|PrintString (Utilities|GetClassDisplayName _returnvalue) true true "(R=1.000000,G=0.993354,B=0.000000,A=1.000000)" 2e+01)
  (if (Utilities|ClassIsChildOf _returnvalue "/Game/VERTICAL_SLICE/BLUEPRINTS/BABIES/BP_Baby.BP_Baby_C")
    (Development|PrintString "SAVED?" true true "(R=1.000000,G=0.993354,B=0.000000,A=1.000000)" 2e+01)
    (Transformation|SetActorLocation OtherActor (Variables|Default|GetsafeZone) false true)
    (else
      (Development|PrintString "FALSE" true true "(R=1.000000,G=0.993354,B=0.000000,A=1.000000)" 2e+01))))

(fn ConstructionScript)