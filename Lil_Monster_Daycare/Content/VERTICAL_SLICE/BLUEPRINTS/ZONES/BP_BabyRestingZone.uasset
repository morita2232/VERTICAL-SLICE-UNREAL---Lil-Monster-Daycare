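; BP_BabyRestingZone is a trigger zone where an overlapping BP_Baby relaxes and has its Anger adjusted.
; On overlap, Chilling sets IsRelaxing, then adds ChillRate to Anger on a delayed loop while Anger stays below MinAnger.
; The loop rechecks Inside only after it ends and latches Chill, which is never reset.
; Leaving clears Inside and prints a debug message, but leaves IsRelaxing set.
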(event OnComponentBeginOverlap(Box)
  (params (OverlappedComponent :type Primitive%20Component%20Object%20Reference) (OtherActor :type Actor%20Object%20Reference) (OtherComp :type Primitive%20Component%20Object%20Reference) (OtherBodyIndex :type Integer) (bFromSweep :type Boolean) (SweepResult :type Hit%20Result%20Structure%20%28by%20ref%29))
  (if (Utilities|ClassIsChildOf (Utilities|GetClass OtherActor) "/Game/VERTICAL_SLICE/BLUEPRINTS/BABIES/BP_Baby.BP_Baby_C")
    (Variables|Default|SetBaby OtherActor)
    (Variables|Default|SetbInside true)
    (CallFunction|Chilling)))

(event OnComponentEndOverlap(Box)
  (params (OverlappedComponent :type Primitive%20Component%20Object%20Reference) (OtherActor :type Actor%20Object%20Reference) (OtherComp :type Primitive%20Component%20Object%20Reference) (OtherBodyIndex :type Integer))
  (if (Utilities|ClassIsChildOf (Utilities|GetClass OtherActor) "/Game/VERTICAL_SLICE/BLUEPRINTS/BABIES/BP_Baby.BP_Baby_C")
    (Variables|Default|SetbInside false)
    (CallFunction|Chilling)))

(event Custom|Chilling
  (if (Variables|Default|GetbInside) :!label _label
    (if (Variables|Default|GetbChill)
      (bind _asbp_baby (Utilities|Casting|CastToBP_Baby (Variables|Default|GetBaby)))
      (Variables|/Game/VERTICAL_SLICE/BLUEPRINTS/BABIES/BP_Baby.BP_Baby_C|SetbIsRelaxing _asbp_baby true)
      (Development|PrintString "Baby chilled out")
      (else
        (bind _asbp_baby_2 (Utilities|Casting|CastToBP_Baby (Variables|Default|GetBaby) :!label _label_2))
        (Variables|/Game/VERTICAL_SLICE/BLUEPRINTS/BABIES/BP_Baby.BP_Baby_C|SetbIsRelaxing _asbp_baby_2 true)
        (bind _output_get (Variables|/Game/VERTICAL_SLICE/BLUEPRINTS/BABIES/BP_Baby.BP_Baby_C|SetAnger _asbp_baby_2 (+ (Variables|/Game/VERTICAL_SLICE/BLUEPRINTS/BABIES/BP_Baby.BP_Baby_C|GetAnger _asbp_baby_2) (Variables|Default|GetchillRate))))
        (Utilities|FlowControl|Delay 15.0)
        (if (< _output_get (Variables|Default|GetminAnger))
          (Development|PrintString "Baby chilling...")
          (goto _label_2)
          (else
            (Variables|Default|SetbChill true)
            (goto _label)))))
    (else
      (Development|PrintString "Baby left resting area"))))

(fn ConstructionScript)