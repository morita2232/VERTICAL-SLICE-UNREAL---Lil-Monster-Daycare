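; Box trigger zone where an overlapping BP_Baby plays until it counts as happy.
; On entry it stores the baby, flags it as playing, then adds FunRate to its Boredom in a delayed loop until MinBoredom is reached.
; Reaching that threshold sets a Happy flag, never reset here, and stops play.
; Exit clears Inside, but the running loop only rechecks it after the threshold is met.
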(event OnComponentBeginOverlap(Box)
  (params (OverlappedComponent :type Primitive%20Component%20Object%20Reference) (OtherActor :type Actor%20Object%20Reference) (OtherComp :type Primitive%20Component%20Object%20Reference) (OtherBodyIndex :type Integer) (bFromSweep :type Boolean) (SweepResult :type Hit%20Result%20Structure%20%28by%20ref%29))
  (if (Utilities|ClassIsChildOf (Utilities|GetClass OtherActor) "/Game/VERTICAL_SLICE/BLUEPRINTS/BABIES/BP_Baby.BP_Baby_C")
    (Variables|Default|SetBaby OtherActor)
    (Variables|Default|SetbInside true)
    (CallFunction|Playing)))

(event OnComponentEndOverlap(Box)
  (params (OverlappedComponent :type Primitive%20Component%20Object%20Reference) (OtherActor :type Actor%20Object%20Reference) (OtherComp :type Primitive%20Component%20Object%20Reference) (OtherBodyIndex :type Integer))
  (if (Utilities|ClassIsChildOf (Utilities|GetClass OtherActor) "/Game/VERTICAL_SLICE/BLUEPRINTS/BABIES/BP_Baby.BP_Baby_C")
    (Variables|Default|SetbInside false)
    (CallFunction|Playing)))

(event Custom|Playing
  (if (Variables|Default|GetbInside) :!label _label
    (if (Variables|Default|GetbHappy)
      (bind _asbp_baby (Utilities|Casting|CastToBP_Baby (Variables|Default|GetBaby)))
      (Variables|/Game/VERTICAL_SLICE/BLUEPRINTS/BABIES/BP_Baby.BP_Baby_C|SetbIsPlaying _asbp_baby false)
      (Development|PrintString "Baby happy!")
      (else
        (bind _asbp_baby_2 (Utilities|Casting|CastToBP_Baby (Variables|Default|GetBaby) :!label _label_2))
        (Variables|/Game/VERTICAL_SLICE/BLUEPRINTS/BABIES/BP_Baby.BP_Baby_C|SetbIsPlaying _asbp_baby_2 true)
        (bind _output_get (Variables|/Game/VERTICAL_SLICE/BLUEPRINTS/BABIES/BP_Baby.BP_Baby_C|SetBoredom _asbp_baby_2 (+ (Variables|/Game/VERTICAL_SLICE/BLUEPRINTS/BABIES/BP_Baby.BP_Baby_C|GetBoredom _asbp_baby_2) (Variables|Default|GetfunRate))))
        (Utilities|FlowControl|Delay 15.0)
        (if (< _output_get (Variables|Default|GetminBoredom))
          (Development|PrintString "Baby playing...")
          (goto _label_2)
          (else
            (Variables|Default|SetbHappy true)
            (goto _label)))))
    (else
      (Development|PrintString "Baby left playing zone"))))

(fn ConstructionScript)