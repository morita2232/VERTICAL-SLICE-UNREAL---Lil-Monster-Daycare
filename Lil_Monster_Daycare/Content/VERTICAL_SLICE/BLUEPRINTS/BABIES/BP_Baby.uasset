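; Baby creature actor that wanders randomly and tracks hunger, boredom and anger.
; Tick interpolates it toward random nearby points unless carried, with timed idle pauses on arrival or sphere hit.
; Looping timers drain each randomly seeded need, playing audio and Niagara for ten seconds when one bottoms out.
; A sphere overlap detects enemy, friend, relative and food classes, doubling anger drain near enemies and hunger drain near food; the others only print debug text.
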(event OnComponentBeginOverlap(Sphere1)
  (params (OverlappedComponent :type Primitive%20Component%20Object%20Reference) (OtherActor :type Actor%20Object%20Reference) (OtherComp :type Primitive%20Component%20Object%20Reference) (OtherBodyIndex :type Integer) (bFromSweep :type Boolean) (SweepResult :type Hit%20Result%20Structure%20%28by%20ref%29))
  (if (== (Utilities|GetClass OtherActor) (Variables|Default|GetEnemy))
    (Variables|Default|SetbEnemyNearby true)
    (Variables|Default|SetangerMulti 2.0)
    (CallFunction|ENEMYCHECK)
    (elif (== (Utilities|GetClass OtherActor) (Variables|Default|GetFriend))
      (Variables|Default|SetbFriendNearby true)
      (CallFunction|FRIENDCHECK)
      (elif (and (!= OtherActor self) (== (Utilities|GetClass OtherActor) (Variables|Default|GetRelative)))
        (Variables|Default|SetbRelativeNearby true)
        (CallFunction|RELATIVECHECK)
        (elif (== (Utilities|GetClass OtherActor) (Variables|Default|GetFood))
          (Variables|Default|SetbFoodNearby true)
          (Variables|Default|SethungerMulti 2.0)
          (CallFunction|FOODCHECK))))))

(event OnComponentEndOverlap(Sphere1)
  (params (OverlappedComponent :type Primitive%20Component%20Object%20Reference) (OtherActor :type Actor%20Object%20Reference) (OtherComp :type Primitive%20Component%20Object%20Reference) (OtherBodyIndex :type Integer))
  (if (== (Utilities|GetClass OtherActor) (Variables|Default|GetEnemy))
    (Variables|Default|SetbEnemyNearby false)
    (Variables|Default|SetangerMulti 1.0)
    (CallFunction|ENEMYCHECK)
    (elif (== (Utilities|GetClass OtherActor) (Variables|Default|GetFriend))
      (Variables|Default|SetbFriendNearby false)
      (CallFunction|FRIENDCHECK)
      (elif (and (!= OtherActor self) (== (Utilities|GetClass OtherActor) (Variables|Default|GetRelative)))
        (Variables|Default|SetbRelativeNearby false)
        (CallFunction|RELATIVECHECK)
        (elif (== (Utilities|GetClass OtherActor) (Variables|Default|GetFood))
          (Variables|Default|SetbFoodNearby false)
          (Variables|Default|SethungerMulti 1.0)
          (CallFunction|FOODCHECK))))))

(event OnComponentHit(Sphere1)
  (params (HitComponent :type Primitive%20Component%20Object%20Reference) (OtherActor :type Actor%20Object%20Reference) (OtherComp :type Primitive%20Component%20Object%20Reference) (NormalImpulse :type Vector :default "0, 0, 0") (Hit :type Hit%20Result%20Structure%20%28by%20ref%29))
  (Variables|Default|SetbIsMoving false)
  (CallFunction|StartIdle))

(event Custom|ENEMY%20CHECK
  (if (Variables|Default|GetbEnemyNearby)
    (Development|PrintString (Utilities|String|Append "Me: " (Utilities|GetObjectName self) ", near enemy: " (Utilities|GetClassDisplayName (Variables|Default|GetEnemy))))
    (else
      (Development|PrintString "Enemy left"))))

(event Custom|FRIEND%20CHECK
  (if (Variables|Default|GetbFriendNearby)
    (Development|PrintString (Utilities|String|Append "Me: " (Utilities|GetObjectName self) ", near friend: " (Utilities|GetClassDisplayName (Variables|Default|GetFriend))))
    (else
      (Development|PrintString "Friend left"))))

(event Custom|RELATIVE%20CHECK
  (if (Variables|Default|GetbRelativeNearby)
    (Development|PrintString (Utilities|String|Append "Me: " (Utilities|GetObjectName self) ", near relative: " (Utilities|GetClassDisplayName (Variables|Default|GetRelative))))
    (else
      (Development|PrintString "Relative left"))))

(event Custom|FOOD%20CHECK
  (if (Variables|Default|GetbFoodNearby)
    (Development|PrintString (Utilities|String|Append "Me: " (Utilities|GetObjectName self) ", near food: " (Utilities|GetClassDisplayName (Variables|Default|GetFood))))
    (else
      (Development|PrintString "Food"))))

(event Custom|GetHungry
  (if (not (Variables|Default|GetbIsEating))
    (if (not (Variables|Default|GetbIsAtMinHunger))
      (bind _output_get (Variables|Default|SetHunger (- (Variables|Default|GetHunger) (* (Variables|Default|GethungerRate) (Variables|Default|GethungerMulti)))))
      (if (> _output_get (Variables|Default|GetminHunger))
        (Variables|Default|SetbIsAtMinHunger false)
        (else
          (Variables|Default|SetbIsAtMinHunger true)
          (Audio|Components|Audio|Play (Variables|Default|GetAudio) 0.0)
          (Components|Activation|Activate (Variables|Default|GetNiagara) false)
          (Utilities|FlowControl|Delay 1e+01)
          (Components|Activation|Deactivate (Variables|Default|GetNiagara))
          (Audio|Components|Audio|Stop (Variables|Default|GetAudio)))))))

(event Custom|GetBored
  (if (not (Variables|Default|GetbIsPlaying))
    (if (not (Variables|Default|GetbIsAtMaxBoredom))
      (bind _output_get (Variables|Default|SetBoredom (- (Variables|Default|GetBoredom) (Variables|Default|GetboredomRate))))
      (if (> _output_get (Variables|Default|GetmaxBoredom))
        (Variables|Default|SetbIsAtMaxBoredom false)
        (else
          (Variables|Default|SetbIsAtMaxBoredom true)
          (Audio|Components|Audio|Play (Variables|Default|GetAudio) 0.0)
          (Components|Activation|Activate (Variables|Default|GetNiagara) false)
          (Utilities|FlowControl|Delay 1e+01)
          (Components|Activation|Deactivate (Variables|Default|GetNiagara))
          (Audio|Components|Audio|Stop (Variables|Default|GetAudio)))))))

(event Custom|GetAngry
  (if (not (Variables|Default|GetbIsRelaxing))
    (if (not (Variables|Default|GetbIsAtMaxAnger))
      (bind _output_get (Variables|Default|SetAnger (- (Variables|Default|GetAnger) (* (Variables|Default|GetangerRate) (Variables|Default|GetangerMulti)))))
      (if (> _output_get (Variables|Default|GetmaxAnger))
        (Variables|Default|SetbIsAtMaxAnger false)
        (else
          (Variables|Default|SetbIsAtMaxAnger true)
          (Audio|Components|Audio|Play (Variables|Default|GetAudio) 0.0)
          (Components|Activation|Activate (Variables|Default|GetNiagara) false)
          (Utilities|FlowControl|Delay 1e+01)
          (Components|Activation|Deactivate (Variables|Default|GetNiagara))
          (Audio|Components|Audio|Stop (Variables|Default|GetAudio)))))))

(event Custom|StartIdle
  (Variables|Default|SetbIsMoving false)
  (Utilities|Time|SetTimerbyEvent (delegate Custom|PickNewDestination) (Math|Random|RandomFloatinRange (Variables|Default|GetIdeMinTime) (Variables|Default|GetIdleMaxTime))))

(event Custom|PickNewDestination
  (bind _returnvalue (Math|Random|RandomUnitVector))
  (Variables|Default|SetTargetLocation (+ (Transformation|GetActorLocation) (* (Math|Vector|MakeVector (.x _returnvalue) (.y _returnvalue) 0.0) (Variables|Default|GetWalkRadius))))
  (Variables|Default|SetbIsMoving true))

(event EventBeginPlay
  (Development|PrintString (Utilities|GetObjectName self))
  (Variables|Default|SetAnger (Math|Random|RandomFloatinRange 8e+01 1e+02))
  (Variables|Default|SetHunger (Math|Random|RandomFloatinRange 7e+01 1e+02))
  (Variables|Default|SetBoredom (Math|Random|RandomFloatinRange 5e+01 1e+02))
  (Utilities|Time|SetTimerbyEvent (delegate Custom|GetHungry) 5.0 true)
  (Utilities|Time|SetTimerbyEvent (delegate Custom|GetBored) 5.0 true)
  (Utilities|Time|SetTimerbyEvent (delegate Custom|GetAngry) 5.0 true)
  (CallFunction|StartIdle))

(event EventTick
  (params (DeltaSeconds :type Float%20%28single-precision%29))
  (if (not (Variables|Default|GetbIsCarried))
    (if (Variables|Default|GetbIsMoving)
      (Transformation|SetActorLocation (Math|Interpolation|VInterpTo (Transformation|GetActorLocation) (Variables|Default|GetTargetLocation) DeltaSeconds (Variables|Default|GetMoveSpeed)) false false)
      (if (< (Math|Vector|Distance(Vector) (Transformation|GetActorLocation) (Variables|Default|GetTargetLocation)) 1e+01)
        (Variables|Default|SetbIsMoving false)
        (CallFunction|StartIdle)))))

(fn ConstructionScript)